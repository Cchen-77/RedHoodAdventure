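; RedHoodGameInstance is the game instance that holds the RedHood character's stats, arrow stats, play time and background music state.
; SetToDefault stops the music and resets the character's health, hit damages, speed, bow power and blood value, plus arrow values and the timer.
; PlayBackgroundSound spawns a 2D sound that persists across level transitions and keeps it for later shutdown.
; IncPlayTime counts seconds and rolls them into minutes.
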(fn SettoDefault
  (CallFunction|ShutupBackgroundSound)
  (CallFunction|SetRedHoodtoDefault)
  (CallFunction|SetArrowtoDefault)
  (CallFunction|SetPlayTimetoDefault))

(fn PlayBackgroundSound
  (params (Sound :type Sound%20Base%20Object%20Reference) (VolumeMultiplier :type Float%20%28single-precision%29))
  (bind _returnvalue (Audio|CreateSound2D Sound VolumeMultiplier 1.0 0.0 0 true))
  (Audio|Components|Audio|Play _returnvalue 0.0)
  (Variables|Default|SetBackgroundmusic _returnvalue))

(fn ShutupBackgroundSound
  (bind _backgroundmusic (Variables|Default|GetBackgroundmusic))
  (if (Utilities|IsValid _backgroundmusic)
    (Audio|Components|Audio|Stop _backgroundmusic)
    (Components|DestroyComponent _backgroundmusic)))

(fn SetPlayTimetoDefault
  (Variables|Default|SetPlayTimeSecond 0)
  (Variables|Default|SetPlayTimeMinute 0))

(fn SetRedHoodtoDefault
  (Variables|Default|SetRedHoodHeavyNormalHitDamage 3.0)
  (Variables|Default|SetRedHoodHeavyExtraHitDamage 3.0)
  (Variables|Default|SetRedHoodLightExtraHitDamage 2.0)
  (Variables|Default|SetRedHoodLightNormalHitDamage 1.0)
  (Variables|Default|SetRedHoodDefalutHealth 2e+01)
  (Variables|Default|SetRedHoodHealth 2e+01)
  (Variables|Default|SetRedHoodMaxWalkSpeed 3e+02)
  (Variables|Default|SetRedHoodDrinkBlood 0.0)
  (Variables|Default|SetRedHoodBowPower 3e+02))

(fn SetArrowtoDefault
  (Variables|Default|SetArrowDamage 1.0)
  (Variables|Default|SetArrowLifetime 3.0))

(fn IncPlayTime
  (Math|Integer|IncrementInt (Variables|Default|GetPlayTimeSecond)
    (:%20%20
      (if (== (Variables|Default|GetPlayTimeSecond) 60)
        (Variables|Default|SetPlayTimeSecond 0)
        (Math|Integer|IncrementInt (Variables|Default|GetPlayTimeMinute))))))