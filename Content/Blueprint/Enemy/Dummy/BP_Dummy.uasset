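; BP_Dummy is an enemy dummy that shows the damage of the latest hit on a text render.
; On hurt, it displays the difference between cached and current health, re-caches health, flags itself as hurting and cancels light and heavy attacks and combos.
; A timeline curve then offsets it along world X as a stun reaction before restoring its original location.
; Tick updates action rotation.
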(event EventBeginPlay
  (Variables|Default|SetHealthCache (Class|BaseCharacter|GetDefaultHealth))
  (Rendering|Components|TextRender|SetText (Variables|Default|GetDamageTextRender) (Utilities|Text|ToText(String) (Utilities|String|MakeLiteralString "DAMAGE:0"))))

(event Collision|EventActorBeginOverlap
  (params (OtherActor :type Actor%20Object%20Reference)))

(event EventTick
  (params (DeltaSeconds :type Float%20%28single-precision%29))
  (Class|BaseCharacter|UpdateActionRotation))

(event EventEnemyHurtFinish
  ;[1 1 1] Hurt
  (Variables|Default|SetIsHurting false))

(event EventEnemyHurt
  ;[1 1 1] Hurt
  (Rendering|Components|TextRender|SetText (Variables|Default|GetDamageTextRender) (Utilities|Text|ToText(String) (Utilities|String|Append (Utilities|String|MakeLiteralString "DAMAGE:") (Utilities|String|ToString(Integer) (Class|KismetMathLibrary|ToInt64(Float) (- (Variables|Default|GetHealthCache) (Variables|Default|GetHealth)))))))
  (Variables|Default|SetHealthCache (Variables|Default|GetHealth))
  (Variables|Default|SetIsHurting true)
  (Variables|Default|SetIsLightAttacking false)
  (Variables|Default|SetIsHeavyAttacking false)
  (Class|BaseEnemy|ResetHeavyAttackCombo)
  (Class|BaseEnemy|ResetLightAttackCombo)
  ;;[1 1 1] Stun
  (Variables|Default|SetLocationCache (Transformation|GetActorLocation))
  (bind _stundis (Timeline|Timeline_0 PlayFromStart)
    (:Update
      (Transformation|SetActorLocation (Math|Vector|MakeVector (+ (* _stundis 2.0) (.x (Variables|Default|GetLocationCache))) (.y (Variables|Default|GetLocationCache)) (.z (Variables|Default|GetLocationCache))) false false))
    (:Finished
      (Transformation|SetActorLocation (Variables|Default|GetLocationCache) false false))))

(fn ConstructionScript)