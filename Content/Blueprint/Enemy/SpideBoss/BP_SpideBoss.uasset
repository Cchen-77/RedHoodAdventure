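; Spider boss enemy for a 2D side-view sprite game, with light and heavy melee attack combos against RedHood.
; Light attacks lunge by impulse and heavy attacks charge through the DragonCar timeline; each combo's last hit adds damage, and timers reset the count.
; HitCheck damages opposing-faction actors in the hitbox and triggers a brief hit stop by zeroing its own time dilation.
; Hurt and death events flash the sprite white and red through timeline-driven material swaps.
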(event EventBeginPlay)

(event Collision|EventActorBeginOverlap
  (params (OtherActor :type Actor%20Object%20Reference)))

(event EventEnemyLightAtk
  ;[1 1 1] LightAttack
  (if (not (Class|BaseEnemy|IsMovementLock))
    (Class|BaseEnemy|ResetHeavyAttackCombo)
    (Utilities|Time|ClearTimerbyFunctionName 0 "ResetLightAttackCombo")
    (Variables|Default|SetHitDamage (Variables|Default|GetLightNormalHitDamage))
    (if (== (Variables|Default|GetLightAttackCombo) (- (Variables|Default|GetMAXLightAttackCombo) 1))
      (Variables|Default|SetHitDamage (+ (Variables|Default|GetHitDamage) (Variables|Default|GetLightExtraHitDamage))))
    (Variables|Default|SetIsLightAttacking true)
    (Physics|AddImpulse (Variables|Character|GetCharacterMovement) (Math|Vector|MakeVector (* (Math|Float|SelectFloat 1.0 -1.0 (== (.yaw (Transformation|GetActorRotation)) 0.0)) 1e+03) 0.0 0.0) true)))

(event EventResetLightAttackCombo
  ;[1 1 1] LightAttack
  (Variables|Default|SetLightAttackCombo 0))

(event EventTick
  (params (DeltaSeconds :type Float%20%28single-precision%29))
  (Class|BaseCharacter|UpdateActionRotation))

(event EventEnemyHeavyAtk
  ;[1 1 1] HeavyAttack
  (if (not (Class|BaseEnemy|IsMovementLock))
    (Class|BaseEnemy|ResetLightAttackCombo)
    (Utilities|Time|ClearTimerbyFunctionName 0 "ResetHeavyAttackCombo")
    (Variables|Default|SetHitDamage (Variables|Default|GetHeavyNormalHitDamage))
    (if (== (Variables|Default|GetHeavyAttackCombo) (- (Variables|Default|GetMAXHeavyAttackCombo) 1))
      (Variables|Default|SetHitDamage (+ (Variables|Default|GetHitDamage) (Variables|Default|GetHeavyExtraHitDamage))))
    (Variables|Default|SetIsHeavyAttacking true)
    (bind _dragoncar (Timeline|DragonCar PlayFromStart)
      (:Update
        (if (> _dragoncar 0.0)
          (Variables|/Script/Engine.MovementComponent|SetVelocity (Variables|Character|GetCharacterMovement) (Math|Vector|MakeVector (* (Variables|Default|GetDragonCarspeed) (select (== (.yaw (Transformation|GetActorRotation)) 0.0) 1.0 -1.0)) (.y (Variables|/Script/Engine.MovementComponent|GetVelocity (Variables|Character|GetCharacterMovement))) (.z (Variables|/Script/Engine.MovementComponent|GetVelocity (Variables|Character|GetCharacterMovement))))))))))

(event EventEnemyHeavyAtkFinish
  ;[1 1 1] HeavyAttack
  (Variables|Default|SetIsHeavyAttacking false)
  (Math|Integer|IncrementInt (Variables|Default|GetHeavyAttackCombo)
    (:%20%20
      (Variables|Default|SetHeavyAttackCombo (Math|Integer|%(Integer) (Variables|Default|GetHeavyAttackCombo) (Variables|Default|GetMAXHeavyAttackCombo)))
      (Utilities|Time|SetTimerbyFunctionName 0 "ResetHeavyAttackCombo" 0.5))))

(event EventResetHeavyAttackCombo
  ;[1 1 1] HeavyAttack
  (Variables|Default|SetHeavyAttackCombo 0))

(event EventEnemyLightAtkFinish
  ;[1 1 1] LightAttack
  (Variables|Default|SetIsLightAttacking false)
  (Math|Integer|IncrementInt (Variables|Default|GetLightAttackCombo)
    (:%20%20
      (Variables|Default|SetLightAttackCombo (Math|Integer|%(Integer) (Variables|Default|GetLightAttackCombo) (Variables|Default|GetMAXLightAttackCombo)))
      (Utilities|Time|SetTimerbyFunctionName 0 "ResetLightAttackCombo" 0.5))))

(event EventEnemyDead
  ;[1 1 1] Dead
  (Variables|Default|SetIsDead true)
  (Variables|Default|SetIsLightAttacking false)
  (Variables|Default|SetIsHeavyAttacking false)
  (Class|BaseEnemy|ResetHeavyAttackCombo)
  (Class|BaseEnemy|ResetLightAttackCombo)
  ;;[1 1 1] HurtFlash
  (bind _lightcolor (Timeline|Timeline_0 PlayFromStart)
    (:Update
      (if (> _lightcolor 0.0)
        (Rendering|Material|SetMaterial (Variables|Default|GetSprite) 0 "/Game/Material/MaskedLitSpriteFlashWhite_MI.MaskedLitSpriteFlashWhite_MI")
        (else
          (Rendering|Material|SetMaterial (Variables|Default|GetSprite) 0 "/Game/Material/MaskedLitSpriteFlashRed_MI.MaskedLitSpriteFlashRed_MI"))))
    (:Finished
      (Rendering|Material|SetMaterial (Variables|Default|GetSprite) 0 "/Paper2D/MaskedLitSpriteMaterial.MaskedLitSpriteMaterial"))))

(event EventEnemyHurt
  ;[1 1 1] Hurt
  ;;[1 1 1] HurtFlash
  (bind _lightcolor (Timeline|HurtFlash PlayFromStart)
    (:Update
      (if (> _lightcolor 0.0)
        (Rendering|Material|SetMaterial (Variables|Default|GetSprite) 0 "/Game/Material/MaskedLitSpriteFlashWhite_MI.MaskedLitSpriteFlashWhite_MI")
        (else
          (Rendering|Material|SetMaterial (Variables|Default|GetSprite) 0 "/Game/Material/MaskedLitSpriteFlashRed_MI.MaskedLitSpriteFlashRed_MI"))))
    (:Finished
      (Rendering|Material|SetMaterial (Variables|Default|GetSprite) 0 "/Paper2D/MaskedLitSpriteMaterial.MaskedLitSpriteMaterial"))))

(event EventHitStop
  ;[1 1 1] HitStop
  (Variables|Default|SetCustomTimeDilation 0.0)
  (Utilities|Time|SetTimerbyFunctionName 0 "HitStopFinish" 0.1))

(event EventHitCheck
  ;[1 1 1] HitCheck
  (Variables|Default|SetHitSth false)
  (for _array_element (Collision|GetOverlappingActors (Variables|Default|GetHitBox) "/Game/Blueprint/Player/RedHood/BP_RedHood.BP_RedHood_C" :!class /Script/Engine.PrimitiveComponent)
    (bind _asbase_character (Utilities|Casting|CastToBaseCharacter _array_element))
    (if (Utilities|Enum|NotEqual(Enum) (Variables|/Script/RedHoodAdventure.BaseCharacter|GetFaction _asbase_character) (Variables|Default|GetFaction self))
      (Game|Damage|ApplyDamage _array_element (Variables|Default|GetHitDamage) 0 self)
      (Variables|Default|SetHitSth true)
      (Variables|Default|SetHitOnce true)))
  (if (Variables|Default|GetHitSth)
    (Class|BaseCharacter|HitStop)))

(event EventHitStopFinish
  ;[1 1 1] HitStop
  (Variables|Default|SetCustomTimeDilation 1.0))

(fn ConstructionScript)