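; Base arrow actor that damages enemies of an opposing faction and destroys itself on a hit.
; On BeginPlay it loads its damage and lifetime from RedHoodGameInstance.
; The HitCheck event, not called within this graph, polls HitBox for overlapping BaseEnemy actors instead of using overlap events.
; It compares each one's Faction to its own and applies damage with the player's BP_RedHood pawn as the causer.
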(event EventBeginPlay
  (CallFunction|LoadData))

(event Collision|EventActorBeginOverlap
  (params (OtherActor :type Actor%20Object%20Reference)))

(event EventTick
  (params (DeltaSeconds :type Float%20%28single-precision%29)))

(event EventHitCheck
  ;[1 1 1] HitCheck
  (Variables|Default|SetHitSth false)
  (for _array_element (Collision|GetOverlappingActors (Variables|Default|GetHitBox) "/Script/RedHoodAdventure.BaseEnemy" :!class /Script/Engine.PrimitiveComponent)
    (bind _asbase_character (Utilities|Casting|CastToBaseCharacter _array_element))
    (if (Utilities|Enum|NotEqual(Enum) (Variables|/Script/RedHoodAdventure.BaseCharacter|GetFaction _asbase_character) (Variables|Default|GetFaction self))
      (bind _asbp_red_hood (Utilities|Casting|CastToBP_RedHood (Game|Player|GetPlayerPawn 0)))
      (Game|Damage|ApplyDamage _array_element (Variables|Default|GetHitDamage) 0 _asbp_red_hood)
      (Variables|Default|SetHitSth true)))
  (if (Variables|Default|GetHitSth)
    (Actor|DestroyActor)))

(fn ConstructionScript)

(fn LoadData
  (bind _asred_hood_game_instance (Utilities|Casting|CastToRedHoodGameInstance (Game|GetGameInstance)))
  (Variables|Default|SetHitDamage (Variables|/Game/Blueprint/RedHoodGameInstance.RedHoodGameInstance_C|GetArrowDamage _asred_hood_game_instance))
  (Variables|Default|SetLifetime (Variables|/Game/Blueprint/RedHoodGameInstance.RedHoodGameInstance_C|GetArrowLifetime _asred_hood_game_instance)))