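; BP_LevelGate is a level exit gate that lets the BP_RedHood character move on to the level named by NextLevelName.
; Its HitCheck event scans HitBox overlaps for BP_RedHood, showing GuideSprite and setting IsOpen while present, hiding and clearing them otherwise.
; The OpenDoor event loads the next level only if IsOpen is set.
; Tick and overlap events are unused, and nothing in this graph calls either custom event.
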(event EventBeginPlay
  (Development|SetHiddeninGame (Variables|Default|GetGuideSprite) true false)
  (Variables|Default|SetIsOpen false))

(event Collision|EventActorBeginOverlap
  (params (OtherActor :type Actor%20Object%20Reference)))

(event EventTick
  (params (DeltaSeconds :type Float%20%28single-precision%29)))

(event EventHitCheck
  ;[1 1 1] HitCheck
  (Variables|Default|SetRedHoodIn false)
  (for _array_element (Collision|GetOverlappingActors (Variables|Default|GetHitBox) "/Script/RedHoodAdventure.BaseCharacter" :!class /Script/Engine.PrimitiveComponent)
    (Utilities|Casting|CastToBP_RedHood _array_element)
    (Variables|Default|SetRedHoodIn true))
  (if (Variables|Default|GetRedHoodIn)
    (Development|SetHiddeninGame (Variables|Default|GetGuideSprite) false false)
    (Variables|Default|SetIsOpen true)
    (else
      (Development|SetHiddeninGame (Variables|Default|GetGuideSprite) true false)
      (Variables|Default|SetIsOpen false))))

(event EventOpenDoor
  ;[1 1 1] OpenDoor
  (if (Variables|Default|GetIsOpen)
    (Game|OpenLevel(byName) (Variables|Default|GetNextLevelName))))

(fn ConstructionScript)